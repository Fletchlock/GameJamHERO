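; HERO game instance that shows a loading screen widget and manages background music with a saved mute preference.
; On Init it adds the widget to the viewport and reads the mute flag from the MusicSlot save.
; StartMusic plays a 2D sound that can persist across levels, applying the mute if set.
; Mute and unmute override the music sound class in HEROSoundMix, while SaveMusicSlot writes the flag back, creating the save if absent.
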(event `self.ReceiveInit`
  (bind _returnvalue (`|CreateWidget` "/Game/UI/WB_LoadingScreen.WB_LoadingScreen_C"))
  (`UserWidget.AddToViewport` _returnvalue 0)
  (set `self.WB_LoadingScreenRef` _returnvalue)
  (bind _returnvalue_2 (`GameplayStatics.DoesSaveGameExist` (`self.MusicSlot`)))
  (if _returnvalue_2
    (bind _returnvalue_3 (`GameplayStatics.LoadGameFromSlot` (`self.MusicSlot`)))
    (bind _output_get (set `self.SaveGameMusicSubClass` _returnvalue_3))
    (bind _assave_game_music (cast `/Game/Blueprints/SaveGameMusic` _output_get))
    (set `self.musicMuted?` (`/Game/Blueprints/SaveGameMusic.musicMuted?` _assave_game_music))))

(fn `Mute Music`
  (`GameplayStatics.SetSoundMixClassOverride` "/Game/Sound/HEROSoundMix.HEROSoundMix" "/Game/Sound/SFX_Music.SFX_Music" 0.0 1.0 0.1)
  (set `self.musicMuted?` true))

(fn `SaveMusicSlot`
  (bind _musicmuted_ (`self.musicMuted?`))
  (bind _returnvalue (`GameplayStatics.DoesSaveGameExist` (`self.MusicSlot`)))
  (if _returnvalue
    (bind _returnvalue_2 (`GameplayStatics.LoadGameFromSlot` (`self.MusicSlot`)))
    (bind _output_get (set `self.SaveGameMusicSubClass` _returnvalue_2))
    (bind _assave_game_music (cast `/Game/Blueprints/SaveGameMusic` _output_get))
    (set `/Game/Blueprints/SaveGameMusic.musicMuted?` _musicmuted_ _assave_game_music)
    (`GameplayStatics.SaveGameToSlot` (`self.SaveGameMusicSubClass`) (`self.MusicSlot`))
    (else
      (bind _returnvalue_3 (`GameplayStatics.CreateSaveGameObject` "/Game/Blueprints/SaveGameMusic.SaveGameMusic_C"))
      (bind _output_get_2 (set `self.SaveGameMusicSubClass` _returnvalue_3))
      (bind _assave_game_music_2 (cast `/Game/Blueprints/SaveGameMusic` _output_get_2))
      (set `/Game/Blueprints/SaveGameMusic.musicMuted?` _musicmuted_ _assave_game_music_2)
      (`GameplayStatics.SaveGameToSlot` (`self.SaveGameMusicSubClass`) (`self.MusicSlot`)))))

(fn `Start Music`
  (params (Music :type "SoundBase Object Reference") (Volume :type "Float (double-precision)") (bPersistAcrossLevelTransition :type Boolean))
  (if (`self.musicMuted?`)
    (bind _returnvalue (`GameplayStatics.CreateSound2D` Music 1.0 1.0 0.0 null bPersistAcrossLevelTransition false))
    (bind _output_get (set `self.MusicAudioComponent` _returnvalue))
    (`self.Mute Music`)
    (`AudioComponent.Play` _output_get 0.0)
    (set `self.musicStarted?` true)
    (else
      (bind _returnvalue_2 (`GameplayStatics.CreateSound2D` Music Volume 1.0 0.0 null bPersistAcrossLevelTransition false))
      (bind _output_get_2 (set `self.MusicAudioComponent` _returnvalue_2))
      (`AudioComponent.Play` _output_get_2 0.0)
      (set `self.musicStarted?` true))))

(fn `Unmute Music`
  (`GameplayStatics.SetSoundMixClassOverride` "/Game/Sound/HEROSoundMix.HEROSoundMix" "/Game/Sound/SFX_Music.SFX_Music" 1.0 1.0 0.1)
  (set `self.musicMuted?` false))
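; BP_MenuSpider is a spider actor, apparently for the menu, that moves its static mesh vertically.
; On BeginPlay it records the mesh's world Z, then plays the SpiderMove timeline, adding its Zvalue to that height while preserving X and Y.
; Each timeline update also sets Points to a fixed value.
; Tick polls the ToBeDestroyed flag and stops the timeline while it is set.
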(event `self.ReceiveBeginPlay`
  (bind _staticmesh (`self.StaticMesh`))
  (bind (_returnvalue_x _returnvalue_y) (`KismetMathLibrary.BreakVector` (`SceneComponent.K2_GetComponentLocation` _staticmesh)))
  (bind (_returnvalue_x_2 _returnvalue_y_2 _returnvalue_z) (`KismetMathLibrary.BreakVector` (`SceneComponent.K2_GetComponentLocation` (`self.StaticMesh`))))
  (`parent.ReceiveBeginPlay`)
  (set `self.Return Value Z` _returnvalue_z)
  (bind (_direction _zvalue) (`Timeline|SpiderMove` :!label _label)
    (:`Update`
      (`SceneComponent.K2_SetWorldLocation` _staticmesh (`KismetMathLibrary.MakeVector` _returnvalue_x _returnvalue_y (+ (`self.Return Value Z`) _zvalue)) false false)
      (set `self.Points` 50))))

(event `self.ReceiveTick`
  (params (DeltaSeconds :type "Float (single-precision)"))
  (`parent.ReceiveTick` DeltaSeconds)
  (if (`self.toBeDestroyed?`)
    (goto _label :!via `Stop`)))

(fn `UserConstructionScript`
  (`parent.UserConstructionScript`))
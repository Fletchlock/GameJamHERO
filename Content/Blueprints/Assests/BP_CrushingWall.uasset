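; BP_CrushingWall is a trap of two walls that move on their Y axis and damage a TEST actor caught by their pain boxes.
; BeginPlay starts CrushingWallsTimeline, whose two tracks drive each wall's relative Y position.
; A Sound event track on the timeline plays a poof cue at a point offset in X from the root.
; Overlapping either pain box applies fixed damage after a cast to TEST.
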(event `self.ReceiveBeginPlay`
  (`self.MoveWalls`))

(event `MoveWalls`
  (bind _wallleft (`self.WallLeft`))
  (bind _wallright (`self.WallRight`))
  (bind (_returnvalue_x _returnvalue_y _returnvalue_z) (`KismetMathLibrary.BreakVector` (`SceneComponent.K2_GetComponentLocation` (`self.DefaultSceneRoot`))))
  (bind (_relativelocation_x _relativelocation_y _relativelocation_z) (`KismetMathLibrary.BreakVector` (`SceneComponent.RelativeLocation` _wallleft)))
  (bind (_relativelocation_x_2 _relativelocation_y_2 _relativelocation_z_2) (`KismetMathLibrary.BreakVector` (`SceneComponent.RelativeLocation` _wallright)))
  (bind (_direction _leftwally _rightwally) (`Timeline|CrushingWallsTimeline` :!via `PlayFromStart`)
    (:`Update`
      (`SceneComponent.K2_SetRelativeLocation` _wallleft (`KismetMathLibrary.MakeVector` _relativelocation_x _leftwally _relativelocation_z) false false)
      (`SceneComponent.K2_SetRelativeLocation` _wallright (`KismetMathLibrary.MakeVector` _relativelocation_x_2 _rightwally _relativelocation_z_2) false false))
    (:`Sound`
      (`GameplayStatics.PlaySoundAtLocation` "/Game/Sound/poof-in-cloud_Cue.poof-in-cloud_Cue" (`KismetMathLibrary.MakeVector` (- _returnvalue_x 4000.0) _returnvalue_y _returnvalue_z) (struct) 1.0 1.0 0.0 null null null))))

(event `self.PainBoxLeft.OnComponentBeginOverlap`
  (params (OverlappedComponent :type "PrimitiveComponent Object Reference") (OtherActor :type "Actor Object Reference") (OtherComp :type "PrimitiveComponent Object Reference") (OtherBodyIndex :type Integer) (bFromSweep :type Boolean) (SweepResult :type "HitResult Structure (by ref)"))
  (bind _astest (cast `/Game/Blueprints/TEST` OtherActor))
  (`GameplayStatics.ApplyDamage` _astest 100.0))

(event `self.PainBoxRight.OnComponentBeginOverlap`
  (params (OverlappedComponent :type "PrimitiveComponent Object Reference") (OtherActor :type "Actor Object Reference") (OtherComp :type "PrimitiveComponent Object Reference") (OtherBodyIndex :type Integer) (bFromSweep :type Boolean) (SweepResult :type "HitResult Structure (by ref)"))
  (bind _astest (cast `/Game/Blueprints/TEST` OtherActor))
  (`GameplayStatics.ApplyDamage` _astest 100.0))

(fn `UserConstructionScript`)
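; BP_TnT is a timed explosive actor that damages what it hits, then destroys itself.
; On BeginPlay a timeline animates a spotlight's cone angles while a short fuse delay runs, then the mesh hides.
; An upward multi-sphere trace applies damage to each hit and sets TnTDone on the player's TEST character.
; Separately, actors overlapping BlastRadius receive OnMessage through the Interact interface.
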(event `self.ReceiveBeginPlay`
  (bind _astest (cast `/Game/Blueprints/TEST` (`GameplayStatics.GetPlayerCharacter` 0)))
  (set `self.As TEST` _astest)
  (`self.BlastLight`)
  (`KismetSystemLibrary.Delay` 1.5)
  (`SceneComponent.SetVisibility` (`self.TnT`) false true)
  (`self.BlastTrace`))

(event `BlastTrace`
  (bind _tnt (`self.TnT`))
  (bind (_returnvalue_x _returnvalue_y _returnvalue_z) (`KismetMathLibrary.BreakVector` (`SceneComponent.K2_GetComponentLocation` _tnt)))
  (bind _outhits (`KismetSystemLibrary.SphereTraceMulti` :`Start` (`SceneComponent.K2_GetComponentLocation` _tnt) :`End` (`KismetMathLibrary.MakeVector` _returnvalue_x _returnvalue_y (+ _returnvalue_z 150.0)) :`Radius` 90.0 :`TraceChannel` "TraceTypeQuery1" :`DrawTime` 0.2))
  (for _array_element _outhits
    (`GameplayStatics.ApplyDamage` (`.HitActor` (`GameplayStatics.BreakHitResult` _array_element)) (`self.Damage`))
    (set `/Game/Blueprints/TEST.bTnTDone?` true (`self.As TEST`)))
  (`self.K2_DestroyActor`))

(event `self.BlastRadius.OnComponentBeginOverlap`
  (params (OverlappedComponent :type "PrimitiveComponent Object Reference") (OtherActor :type "Actor Object Reference") (OtherComp :type "PrimitiveComponent Object Reference") (OtherBodyIndex :type Integer) (bFromSweep :type Boolean) (SweepResult :type "HitResult Structure (by ref)"))
  (if (`KismetSystemLibrary.DoesImplementInterface` OtherActor "/Game/Blueprints/Interact.Interact_C")
    (message `/Game/Blueprints/Interact.On` OtherActor)))

(event `BlastLight`
  (bind _spotlight (`self.SpotLight`))
  (bind (_direction _radius) (`Timeline|BlastLightTL` :!via `PlayFromStart`)
    (:`Update`
      (`SpotLightComponent.SetInnerConeAngle` _spotlight _radius)
      (`SpotLightComponent.SetOuterConeAngle` _spotlight _radius))))

(fn `UserConstructionScript`)
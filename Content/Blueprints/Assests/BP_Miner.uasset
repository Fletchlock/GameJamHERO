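; BP_Miner is a rescuable miner that ends the level when the TEST character overlaps its Box.
; On overlap it sets EndLevel, disables the character's movement, turns its mesh to 90 yaw and freezes its animation.
; It then plays the rescue animation and spawns a BP_PointsText above the miner showing Points.
; The player cached at BeginPlay receives its own MinerScore and recalculates score.
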(event `self.ReceiveBeginPlay`
  (bind _astest (cast `/Game/Blueprints/TEST` (`GameplayStatics.GetPlayerCharacter` 0)))
  (set `self.As TEST` _astest))

(event `self.Box.OnComponentBeginOverlap`
  (params (OverlappedComponent :type "PrimitiveComponent Object Reference") (OtherActor :type "Actor Object Reference") (OtherComp :type "PrimitiveComponent Object Reference") (OtherBodyIndex :type Integer) (bFromSweep :type Boolean) (SweepResult :type "HitResult Structure (by ref)"))
  (bind _as_test (`self.As TEST`))
  (bind (_returnvalue_x _returnvalue_y _returnvalue_z) (`KismetMathLibrary.BreakVector` (`SceneComponent.K2_GetComponentLocation` (`self.Miner`))))
  (bind _astest (cast `/Game/Blueprints/TEST` OtherActor))
  (set `/Game/Blueprints/TEST.endLevel?` true _astest)
  (`CharacterMovementComponent.DisableMovement` (`Character.CharacterMovement` _astest))
  (bind _mesh (`Character.Mesh` _astest))
  (bind (_returnvalue_roll _returnvalue_pitch) (`KismetMathLibrary.BreakRotator` (`SceneComponent.K2_GetComponentRotation` _mesh)))
  (`SceneComponent.K2_SetWorldRotation` _mesh (`KismetMathLibrary.MakeRotator` _returnvalue_roll _returnvalue_pitch 90.0) false false)
  (set `SkeletalMeshComponent.GlobalAnimRateScale` 0.0 _mesh)
  (`SkeletalMeshComponent.PlayAnimation` (`self.Miner`) "/Game/Miner/Animations/MinerRescue.MinerRescue" false)
  (bind _returnvalue (`|SpawnActorFromClass` "/Game/Blueprints/Assests/BP_PointsText.BP_PointsText_C" (`KismetMathLibrary.MakeTransform` (`KismetMathLibrary.MakeVector` _returnvalue_x _returnvalue_y (+ _returnvalue_z 100.0))) "Undefined" "OverrideRootScale" null null))
  (`/Game/Blueprints/Assests/BP_PointsText.ShowPointsText` _returnvalue (`self.Points`))
  (set `/Game/Blueprints/TEST.Score` (+ (`/Game/Blueprints/TEST.Score` _as_test) (`/Game/Blueprints/TEST.MinerScore` _as_test)) (`self.As TEST`))
  (`/Game/Blueprints/TEST.CalcScore` (`self.As TEST`)))

(fn `UserConstructionScript`)
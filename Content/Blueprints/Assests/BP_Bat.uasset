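; BP_Bat is a flying enemy that bobs vertically and damages the actor referenced by AsTEST on contact.
; The SnakeYMove timeline, paced by that actor's PlaybackSpeed, offsets the mesh and box height from the starting Z and sets the Points value.
; Box1 overlap applies damage, sets ToBeDestroyed, spawns a Niagara burst and destroys the bat.
; Tick watches ToBeDestroyed to change the animation and stop the timeline.
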(event `self.ReceiveBeginPlay`
  (bind (_returnvalue_x _returnvalue_y _returnvalue_z) (`KismetMathLibrary.BreakVector` (`SceneComponent.K2_GetComponentLocation` (`self.StaticMesh`))))
  (bind (_returnvalue_x_2 _returnvalue_y_2) (`KismetMathLibrary.BreakVector` (`SceneComponent.K2_GetComponentLocation` (`self.Box`))))
  (`parent.ReceiveBeginPlay`)
  (set `self.Return Value z` _returnvalue_z)
  (`KismetSystemLibrary.Delay` 0.1)
  (`TimelineComponent.SetPlayRate` (`self.SnakeYMove`) (`/Game/Blueprints/TEST.PlaybackSpeed` (`self.As TEST`)))
  (bind (_direction _yvalue) (`Timeline|SnakeYMove` :!label _label)
    (:`Update`
      (`SceneComponent.K2_SetWorldLocation` (`self.StaticMesh`) (`KismetMathLibrary.MakeVector` _returnvalue_x_2 _returnvalue_y_2 (+ (`self.Return Value z`) _yvalue)) false false)
      (`SceneComponent.K2_SetWorldLocation` (`self.Box`) (`KismetMathLibrary.MakeVector` _returnvalue_x_2 _returnvalue_y_2 (+ (`self.Return Value z`) _yvalue)) false false)
      (set `self.Points` 50))))

(event `self.ReceiveTick`
  (params (DeltaSeconds :type "Float (single-precision)"))
  (`parent.ReceiveTick` DeltaSeconds)
  (if (`self.toBeDestroyed?`)
    (`SkeletalMeshComponent.SetAnimation` (`self.SkeletalMesh`) null)
    (goto _label :!via `Stop`)))

(event `self.Box1.OnComponentBeginOverlap`
  (params (OverlappedComponent :type "PrimitiveComponent Object Reference") (OtherActor :type "Actor Object Reference") (OtherComp :type "PrimitiveComponent Object Reference") (OtherBodyIndex :type Integer) (bFromSweep :type Boolean) (SweepResult :type "HitResult Structure (by ref)"))
  (if (== (`self.As TEST`) OtherActor)
    (`GameplayStatics.ApplyDamage` (`self.As TEST`) 10.0)
    (set `self.toBeDestroyed?` true)
    (`NiagaraFunctionLibrary.SpawnSystemAtLocation` "/Game/Blueprints/HeroFX/NS_BurstingBaddie.NS_BurstingBaddie" (`SceneComponent.K2_GetComponentLocation` (`self.Box`)))
    (`self.K2_DestroyActor`)))

(fn `UserConstructionScript`
  (`parent.UserConstructionScript`))
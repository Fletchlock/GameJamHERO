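; BP_MenuSnake is a snake actor, apparently for the menu, that moves along the Y axis and carries a point value.
; On BeginPlay it caches the box's world Y and plays the SnakeYMove timeline, which offsets the box from that start and sets Points on each update.
; Tick polls ToBeDestroyed and, while it is true, calls SetAnimation on the skeletal mesh and stops the timeline.
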(event `self.ReceiveBeginPlay`
  (bind _box (`self.Box`))
  (bind (_returnvalue_x _returnvalue_y) (`KismetMathLibrary.BreakVector` (`SceneComponent.K2_GetComponentLocation` (`self.Box`))))
  (bind (_returnvalue_x_2 _returnvalue_y_2 _returnvalue_z) (`KismetMathLibrary.BreakVector` (`SceneComponent.K2_GetComponentLocation` _box)))
  (`parent.ReceiveBeginPlay`)
  (set `self.Return Value Y` _returnvalue_y)
  (bind (_direction _yvalue) (`Timeline|SnakeYMove` :!label _label)
    (:`Update`
      (`SceneComponent.K2_SetWorldLocation` _box (`KismetMathLibrary.MakeVector` _returnvalue_x_2 (+ (`self.Return Value Y`) _yvalue) _returnvalue_z) false false)
      (set `self.Points` 50))))

(event `self.ReceiveTick`
  (params (DeltaSeconds :type "Float (single-precision)"))
  (`parent.ReceiveTick` DeltaSeconds)
  (if (`self.toBeDestroyed?`)
    (`SkeletalMeshComponent.SetAnimation` (`self.SkeletalMesh`) null)
    (goto _label :!via `Stop`)))

(fn `UserConstructionScript`
  (`parent.UserConstructionScript`))
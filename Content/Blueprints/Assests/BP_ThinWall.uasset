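; BP_ThinWall is a destructible thin wall that awards score to the player when destroyed.
; AnyDamage drains Health; at zero it adds a fixed score to the cached TEST player character and checks the high score.
; It then spawns a BP_PointsText popup showing Points and a blast smoke Niagara effect before destroying itself.
; On and Off events swap visibility between the normal and dark wall components.
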(event `self.ReceiveBeginPlay`
  (bind _astest (cast `/Game/Blueprints/TEST` (`GameplayStatics.GetPlayerCharacter` 0)))
  (set `self.As TEST` _astest))

(event `self.ReceiveAnyDamage`
  (params (Damage :type "Float (single-precision)") (DamageType :type "DamageType Object Reference") (InstigatedBy :type "Controller Object Reference") (DamageCauser :type "Actor Object Reference"))
  (bind _as_test (`self.As TEST`))
  (bind (_returnvalue_x _returnvalue_y _returnvalue_z) (`KismetMathLibrary.BreakVector` (`SceneComponent.K2_GetComponentLocation` (`self.ThinWall`))))
  (bind (_returnvalue_x_2 _returnvalue_y_2 _returnvalue_z_2) (`KismetMathLibrary.BreakVector` (`SceneComponent.K2_GetComponentLocation` (`self.ThinWall`))))
  (bind _output_get (set `self.Health` (- (`self.Health`) Damage)))
  (if (<= _output_get 0.0)
    (set `/Game/Blueprints/TEST.Score` (+ (`/Game/Blueprints/TEST.Score` _as_test) 75) _as_test)
    (`/Game/Blueprints/TEST.CheckHighScore` _as_test)
    (bind _returnvalue (`|SpawnActorFromClass` "/Game/Blueprints/Assests/BP_PointsText.BP_PointsText_C" (`KismetMathLibrary.MakeTransform` (`KismetMathLibrary.MakeVector` _returnvalue_x _returnvalue_y (+ _returnvalue_z 100.0))) "Undefined" "OverrideRootScale" null null))
    (`/Game/Blueprints/Assests/BP_PointsText.ShowPointsText` _returnvalue (`self.Points`))
    (`NiagaraFunctionLibrary.SpawnSystemAtLocation` "/Game/Blueprints/HeroFX/NS_BlastSmoke.NS_BlastSmoke" (`KismetMathLibrary.MakeVector` _returnvalue_x_2 _returnvalue_y_2 (- _returnvalue_z_2 10.0)))
    (`self.K2_DestroyActor`)))

(event `/Game/Blueprints/Interact.On`
  (bind _thinwalldark (`self.ThinWallDark`))
  (`SceneComponent.SetHiddenInGame` (`self.ThinWall`) false false)
  (`SceneComponent.SetVisibility` _thinwalldark false false)
  (`SceneComponent.SetHiddenInGame` _thinwalldark true false))

(event `/Game/Blueprints/Interact.Off`
  (bind _thinwalldark (`self.ThinWallDark`))
  (`SceneComponent.SetHiddenInGame` (`self.ThinWall`) true false)
  (`SceneComponent.SetVisibility` _thinwalldark true false)
  (`SceneComponent.SetHiddenInGame` _thinwalldark false false))

(fn `UserConstructionScript`)
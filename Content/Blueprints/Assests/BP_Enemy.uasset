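; Enemy actor that awards points when damaged and hurts the player on contact.
; On BeginPlay it caches the TEST player character and copies its playback speed.
; The first damage event plays a gore sound, notifies the player of the kill and spawns floating points text.
; Player overlap with the Box applies damage and skips the reward, joining the same Niagara burst and destroy path.
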(event `self.ReceiveBeginPlay`
  (bind _astest (cast `/Game/Blueprints/TEST` (`GameplayStatics.GetPlayerCharacter` 0)))
  (bind _output_get (set `self.As TEST` _astest))
  (bind _output_get_2 (set `self.Playback Speed` (`/Game/Blueprints/TEST.PlaybackSpeed` _output_get)))
  (set `self.TimelinePlaybackSpeed` _output_get_2)
  (set `self.toBeDestroyed?` false))

(event `self.ReceiveAnyDamage`
  (params (Damage :type "Float (single-precision)") (DamageType :type "DamageType Object Reference") (InstigatedBy :type "Controller Object Reference") (DamageCauser :type "Actor Object Reference"))
  (bind (_returnvalue_x _returnvalue_y _returnvalue_z) (`KismetMathLibrary.BreakVector` (`SceneComponent.K2_GetComponentLocation` (`self.Box`))))
  (`/Engine/EditorBlueprintResources/StandardMacros.DoOnce` false
    (:`Completed`
      (`GameplayStatics.PlaySound2D` "/Game/Sound/gushing-flesh_Cue.gushing-flesh_Cue" 1.0 1.0 0.0 null null)
      (`/Game/Blueprints/TEST.KilledEnemy` (`self.As TEST`))
      (bind _returnvalue (`|SpawnActorFromClass` "/Game/Blueprints/Assests/BP_PointsText.BP_PointsText_C" (`KismetMathLibrary.MakeTransform` (`KismetMathLibrary.MakeVector` _returnvalue_x _returnvalue_y (+ _returnvalue_z 40.0))) "Undefined" "OverrideRootScale" null null))
      (`/Game/Blueprints/Assests/BP_PointsText.ShowPointsText` _returnvalue (`self.Points`))
      (`NiagaraFunctionLibrary.SpawnSystemAtLocation` "/Game/Blueprints/HeroFX/NS_BurstingBaddie.NS_BurstingBaddie" (`SceneComponent.K2_GetComponentLocation` (`self.Box`)) :!label _label)
      (`self.K2_DestroyActor`))))

(event `self.Box.OnComponentBeginOverlap`
  (params (OverlappedComponent :type "PrimitiveComponent Object Reference") (OtherActor :type "Actor Object Reference") (OtherComp :type "PrimitiveComponent Object Reference") (OtherBodyIndex :type Integer) (bFromSweep :type Boolean) (SweepResult :type "HitResult Structure (by ref)"))
  (if (== (`self.As TEST`) OtherActor)
    (`GameplayStatics.ApplyDamage` (`self.As TEST`) 10.0)
    (set `self.toBeDestroyed?` true)
    (goto _label)))

(fn `UserConstructionScript`)
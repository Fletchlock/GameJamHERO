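; BP_LavaWall is a destructible hazard wall that damages the player and awards score when destroyed.
; It caches the player character as TEST on BeginPlay and applies damage to it when it begins overlapping the Box component.
; Incoming damage lowers its health; at zero it adds score, checks the high score, spawns floating points text and blast smoke at the wall, then destroys itself.
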(event `self.ReceiveBeginPlay`
  (bind _astest (cast `/Game/Blueprints/TEST` (`GameplayStatics.GetPlayerCharacter` 0)))
  (set `self.As TEST_0` _astest))

(event `self.ReceiveAnyDamage`
  (params (Damage :type "Float (single-precision)") (DamageType :type "DamageType Object Reference") (InstigatedBy :type "Controller Object Reference") (DamageCauser :type "Actor Object Reference"))
  (bind _as_test_0 (`self.As TEST_0`))
  (bind (_returnvalue_x _returnvalue_y _returnvalue_z) (`KismetMathLibrary.BreakVector` (`SceneComponent.K2_GetComponentLocation` (`self.ThinWall_0`))))
  (bind (_returnvalue_x_2 _returnvalue_y_2 _returnvalue_z_2) (`KismetMathLibrary.BreakVector` (`SceneComponent.K2_GetComponentLocation` (`self.ThinWall_0`))))
  (bind _output_get (set `self.Health_0` (- (`self.Health_0`) Damage)))
  (if (<= _output_get 0.0)
    (set `/Game/Blueprints/TEST.Score` (+ (`/Game/Blueprints/TEST.Score` _as_test_0) 75) _as_test_0)
    (`/Game/Blueprints/TEST.CheckHighScore` _as_test_0)
    (bind _returnvalue (`|SpawnActorFromClass` "/Game/Blueprints/Assests/BP_PointsText.BP_PointsText_C" (`KismetMathLibrary.MakeTransform` (`KismetMathLibrary.MakeVector` _returnvalue_x_2 _returnvalue_y_2 (+ _returnvalue_z_2 100.0))) "Undefined" "OverrideRootScale" null null))
    (`/Game/Blueprints/Assests/BP_PointsText.ShowPointsText` _returnvalue (`self.Points`))
    (`NiagaraFunctionLibrary.SpawnSystemAtLocation` "/Game/Blueprints/HeroFX/NS_BlastSmoke.NS_BlastSmoke" (`KismetMathLibrary.MakeVector` _returnvalue_x _returnvalue_y (- _returnvalue_z 10.0)))
    (`self.K2_DestroyActor`)))

(event `self.Box.OnComponentBeginOverlap`
  (params (OverlappedComponent :type "PrimitiveComponent Object Reference") (OtherActor :type "Actor Object Reference") (OtherComp :type "PrimitiveComponent Object Reference") (OtherBodyIndex :type Integer) (bFromSweep :type Boolean) (SweepResult :type "HitResult Structure (by ref)"))
  (if (== (`self.As TEST_0`) OtherActor)
    (`GameplayStatics.ApplyDamage` (`self.As TEST_0`) 10.0)))

(fn `UserConstructionScript`)
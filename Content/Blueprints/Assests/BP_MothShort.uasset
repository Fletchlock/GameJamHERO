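; BP_MothShort is a moth hazard that flies a timeline-driven path, damages the AsTEST actor on contact and dies.
; The SnakeYMove timeline, paced by that actor's PlaybackSpeed, offsets mesh and box in Y/Z from their start, sets Points and flips skeletal mesh yaw.
; Box1 overlap applies damage, spawns a Niagara burst and destroys the moth after a brief delay, while Tick halts movement once flagged.
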(event `self.ReceiveBeginPlay`
  (bind (_returnvalue_x _returnvalue_y _returnvalue_z) (`KismetMathLibrary.BreakVector` (`SceneComponent.K2_GetComponentLocation` (`self.StaticMesh`))))
  (bind _returnvalue_x_2 (`KismetMathLibrary.BreakVector` (`SceneComponent.K2_GetComponentLocation` (`self.Box`))))
  (`parent.ReceiveBeginPlay`)
  (set `self.Return Value z` _returnvalue_z)
  (set `self.Return Value Y` _returnvalue_y)
  (`KismetSystemLibrary.Delay` 0.1)
  (`TimelineComponent.SetPlayRate` (`self.SnakeYMove`) (`/Game/Blueprints/TEST.PlaybackSpeed` (`self.As TEST`)))
  (bind (_direction _yvalue _zvalue) (`Timeline|SnakeYMove` :!label _label)
    (:`Update`
      (`SceneComponent.K2_SetWorldLocation` (`self.StaticMesh`) (`KismetMathLibrary.MakeVector` _returnvalue_x_2 (+ (`self.Return Value Y`) _yvalue) (+ (`self.Return Value z`) _zvalue)) false false)
      (`SceneComponent.K2_SetWorldLocation` (`self.Box`) (`KismetMathLibrary.MakeVector` _returnvalue_x_2 (+ (`self.Return Value Y`) _yvalue) (+ (`self.Return Value z`) _zvalue)) false false)
      (set `self.Points` 50))
    (:`Rotate`
      (`SceneComponent.K2_SetWorldRotation` (`self.SkeletalMesh`) (`KismetMathLibrary.MakeRotator` 0.0 0.0 90.0) false false))
    (:`Rotate2`
      (`SceneComponent.K2_SetWorldRotation` (`self.SkeletalMesh`) (`KismetMathLibrary.MakeRotator` 0.0 0.0 -90.0) false false))))

(event `self.ReceiveTick`
  (params (DeltaSeconds :type "Float (single-precision)"))
  (`parent.ReceiveTick` DeltaSeconds)
  (if (`self.toBeDestroyed?`)
    (`SkeletalMeshComponent.SetAnimation` (`self.SkeletalMesh`) null)
    (goto _label :!via `Stop`)))

(event `self.Box1.OnComponentBeginOverlap`
  (params (OverlappedComponent :type "PrimitiveComponent Object Reference") (OtherActor :type "Actor Object Reference") (OtherComp :type "PrimitiveComponent Object Reference") (OtherBodyIndex :type Integer) (bFromSweep :type Boolean) (SweepResult :type "HitResult Structure (by ref)"))
  (if (== (`self.As TEST`) OtherActor)
    (`GameplayStatics.ApplyDamage` (`self.As TEST`) 10.0)
    (set `self.toBeDestroyed?` true)
    (`NiagaraFunctionLibrary.SpawnSystemAtLocation` "/Game/Blueprints/HeroFX/NS_BurstingBaddie.NS_BurstingBaddie" (`SceneComponent.K2_GetComponentLocation` (`self.Box`)))
    (`KismetSystemLibrary.Delay` 0.2)
    (`self.K2_DestroyActor`)))

(fn `UserConstructionScript`
  (`parent.UserConstructionScript`))